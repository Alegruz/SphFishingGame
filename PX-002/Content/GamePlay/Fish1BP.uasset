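; Fish actor that spawns at a random spot and wanders horizontally between random destinations within a square range.
; Tick moves it along a normalized direction, faces it that way, and picks a new destination once it is nearly there.
; Jump starts a countdown timer that drives a quadratic per-frame Z offset, which is also printed for debugging.
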(event EventBeginPlay
  (bind _randommin (Variables|Default|GetRandomMin))
  (bind _randommax (Variables|Default|GetRandomMax))
  (Transformation|SetWorldLocation (Variables|Default|GetDefaultSceneRoot) (Math|Vector|MakeVector (Math|Random|RandomFloatinRange _randommin _randommax) (Math|Random|RandomFloatinRange _randommin _randommax) (Math|Random|RandomFloatinRange 2e+01 25.0)) false false))

(event EventTick
  (params (DeltaSeconds :type Float%20%28single-precision%29))
  (bind _returnvalue (Transformation|GetActorLocation))
  (bind _defaultsceneroot (Variables|Default|GetDefaultSceneRoot))
  (if (>= (Variables|Default|GetJumpTimer) 0.0)
    (Variables|Default|SetJumpTimer (- (Variables|Default|GetJumpTimer) DeltaSeconds)))
  (if (Variables|Default|GetMakeDestinationVector)
    (bind (_destination _direction) (CallFunction|MakeRandomDestination))
    (Variables|Default|SetDestinationVector _destination)
    (Variables|Default|SetDirectionVector _direction)
    (Variables|Default|SetMakeDestinationVector false)
    (else
      (Transformation|SetWorldLocation _defaultsceneroot (+ (Transformation|GetActorLocation) (* (Variables|Default|GetDirectionVector) (* (Variables|Default|GetSpeed) DeltaSeconds))) false false)
      (Transformation|SetWorldRotation _defaultsceneroot (Math|Conversions|RotationFromXVector (Variables|Default|GetDirectionVector)) false false)
      (if (>= (Variables|Default|GetJumpTimer) 0.0)
        (Development|PrintString (Utilities|String|ToString(Float) (* (* (* (Variables|Default|GetJumpTimer) (- (Variables|Default|GetJumpTimer) 1e+03)) 4e+01) DeltaSeconds))))
      (Transformation|SetActorLocation (Math|Vector|MakeVector (.x _returnvalue) (.y _returnvalue) (+ (.z _returnvalue) (select (>= (Variables|Default|GetJumpTimer) 0.0) (* (* (* (Variables|Default|GetJumpTimer) (- (Variables|Default|GetJumpTimer) 1e+03)) 4e+01) DeltaSeconds) 0.0))) false false)
      (Variables|Default|SetMakeDestinationVector (Math|Vector|VectorIsNearlyZero (- (Transformation|GetActorLocation) (Variables|Default|GetDestinationVector)) 1e+02)))))

(fn ConstructionScript)

(fn MakeRandomDestination
  (bind _returnvalue (Transformation|GetActorLocation))
  (bind _randommin (Variables|Default|GetRandomMin))
  (bind _randommax (Variables|Default|GetRandomMax))
  (bind _returnvalue_2 (Math|Random|RandomFloatinRange _randommin _randommax))
  (bind _returnvalue_3 (Math|Random|RandomFloatinRange _randommin _randommax))
  (bind _returnvalue_4 (Math|Vector|MakeVector _returnvalue_2 _returnvalue_3 0.0))
  (bind (_x _y) (Math|Vector|BreakVector _returnvalue_4))
  (return _returnvalue_4 (Math|Vector|Normalize (Math|Vector|MakeVector (- _x (.x _returnvalue)) (- _y (.y _returnvalue)) 0.0) 1.0)))

(fn Jump
  (Variables|Default|SetJumpTimer 1e+03))